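; BP_DynamicDayNight is an early stub of a day/night actor, with no cycle or lighting logic in its graphs.
; Its construction script teleports DayIndicator and NightIndicator to a fixed world Y and height, preserving each one's X position.
; Tick and EditorTick only print debug strings to distinguish runtime from in-editor ticking.
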(event EventBeginPlay)

(event EventTick
  (params (DeltaSeconds :type Float%20%28single-precision%29))
  (Development|PrintString "nbormawl tick"))

(event EventEditorTick
  (params (DeltaSeconds :type Float%20%28single-precision%29))
  (Development|PrintString "EDITOR TICK"))

(fn ConstructionScript
  (bind _nightindicator (Variables|Default|GetNightIndicator))
  (bind _dayindicator (Variables|Default|GetDayIndicator))
  (Utilities|FlowControl|Sequence
    (:then_0
      (Transformation|SetWorldLocation _dayindicator (Math|Vector|MakeVector (.X (Math|Vector|BreakVector (Transformation|GetWorldLocation _dayindicator))) 0.0 1e+02) false true))
    (:then_1
      (Transformation|SetWorldLocation _nightindicator (Math|Vector|MakeVector (.X (Math|Vector|BreakVector (Transformation|GetWorldLocation _nightindicator))) 0.0 1e+02) false true))))